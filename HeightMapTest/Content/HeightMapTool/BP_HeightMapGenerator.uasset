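; BP_HeightMapGenerator bakes a world height map at play start, plus blurred and occlusion versions derived from it.
; After clearing its render targets and a brief delay, it triggers a scene capture, then has HeightMapGenerator compute world-to-heightmap mapping parameters.
; It publishes those to a material parameter collection, then draws blur and occlusion materials into their render targets as a one-shot pass with no Tick logic.
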(event `self.ReceiveBeginPlay`
  (bind _heightmapgenerator (`self.HeightMapGenerator`))
  (`KismetRenderingLibrary.ClearRenderTarget2D` "/Game/HeightMapTool/RT_Heightmap.RT_Heightmap" (struct :`R` 0.051551 :`G` 0.984375 :`B` 0.10349 :`A` 1.0))
  (`KismetRenderingLibrary.ClearRenderTarget2D` "/Game/HeightMapTool/RT_Heightmap_Blurred.RT_Heightmap_Blurred")
  (`KismetRenderingLibrary.ClearRenderTarget2D` "/Game/HeightMapTool/RT_OcclusionMap.RT_OcclusionMap")
  (`KismetSystemLibrary.Delay` 0.2)
  (`SceneCaptureComponent2D.CaptureScene` (`self.SceneCaptureComponent2D`))
  (`HeightMapGeneratorComponent.CalcShaderParameters` _heightmapgenerator)
  (`KismetMaterialLibrary.SetVectorParameterValue` "/Game/HeightMapTool/Materials/HeightMapMaterialParameterCollection.HeightMapMaterialParameterCollection" "OffsetAndScale" (`HeightMapGeneratorComponent.World2HeightmapOffsetAndScale` _heightmapgenerator))
  (`KismetMaterialLibrary.SetScalarParameterValue` "/Game/HeightMapTool/Materials/HeightMapMaterialParameterCollection.HeightMapMaterialParameterCollection" "HeightMap2WorldZAdd" (`HeightMapGeneratorComponent.HeightMap2WorldZAdd` _heightmapgenerator))
  (`KismetMaterialLibrary.SetScalarParameterValue` "/Game/HeightMapTool/Materials/HeightMapMaterialParameterCollection.HeightMapMaterialParameterCollection" "HeightMap2WorldZMul" (`HeightMapGeneratorComponent.HeightMap2WorldZMul` _heightmapgenerator))
  (`KismetRenderingLibrary.DrawMaterialToRenderTarget` "/Game/HeightMapTool/RT_Heightmap_Blurred.RT_Heightmap_Blurred" "/Game/HeightMapTool/Materials/MT_PP_Blur.MT_PP_Blur")
  (`KismetRenderingLibrary.DrawMaterialToRenderTarget` "/Game/HeightMapTool/RT_OcclusionMap.RT_OcclusionMap" "/Game/HeightMapTool/Materials/MT_PP_CalcOcclusion_New_Inst.MT_PP_CalcOcclusion_New_Inst"))

(event `self.ReceiveTick`
  (params (DeltaSeconds :type "Float (single-precision)")))

(fn `UserConstructionScript`)